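; BP_VR_Capture_Manager drives the scene captures that provide the views for a pair of VR portals.
; Each tick, a FlipFlop captures only one of the two scene captures, alternating them so each updates every other frame.
; After that capture, if both portals are valid, each capture is moved to the opposite portal's location and oriented from that portal's remapped axes, independent of any player camera.
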(event `self.ReceiveTick`
  (params (DeltaSeconds :type "Float (single-precision)"))
  (bind _scenecapture_portal2 (`self.SceneCapture_Portal2`))
  (bind _portal2 (`self.Portal2`))
  (bind _scenecapture_portal1 (`self.SceneCapture_Portal1`))
  (bind _portal1 (`self.Portal1`))
  (`|ExecutionSequence`
    (:`then_0`
      (`/Engine/EditorBlueprintResources/StandardMacros.FlipFlop`
        (:`A`
          (`SceneCaptureComponent2D.CaptureScene` (`self.SceneCapture_Portal1`)))
        (:`B`
          (`SceneCaptureComponent2D.CaptureScene` (`self.SceneCapture_Portal2`)))))
    (:`then_1`
      (`/Engine/EditorBlueprintResources/StandardMacros.IsValid` (`self.Portal1`)
        (:`Is Valid`
          (`/Engine/EditorBlueprintResources/StandardMacros.IsValid` _portal2
            (:`Is Valid`
              (`|ExecutionSequence`
                (:`then_0`
                  (`SceneComponent.K2_SetWorldLocation` _scenecapture_portal1 (`self.K2_GetActorLocation` _portal2) false true)
                  (`SceneComponent.K2_SetWorldRotation` _scenecapture_portal1 (`KismetMathLibrary.MakeRotationFromAxes` (`self.GetActorUpVector` _portal2) (* (`self.GetActorRightVector` _portal2) -1.0) (`self.GetActorForwardVector` _portal2)) false false))
                (:`then_1`
                  (`SceneComponent.K2_SetWorldLocation` _scenecapture_portal2 (`self.K2_GetActorLocation` _portal1) false true)
                  (`SceneComponent.K2_SetWorldRotation` _scenecapture_portal2 (`KismetMathLibrary.MakeRotationFromAxes` (`self.GetActorUpVector` _portal1) (* (`self.GetActorRightVector` _portal1) -1.0) (`self.GetActorForwardVector` _portal1)) false false))))))))))

(fn `UserConstructionScript`)
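; BP_Tutorial_door is a double sliding door for the tutorial that opens when its OpenDoor event is called.
; OpenDoor plays a sound at the actor and runs the MoveDoors timeline, which slides LeftDoor and RightDoor apart along local X.
; Each update lerps from the current location to a fixed offset, so motion compounds rather than following the curve directly.
; When finished, both doors ignore all collision channels; no close logic exists.
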(event `OpenDoor`
  (bind _leftdoor (`self.LeftDoor`))
  (bind _rightdoor (`self.RightDoor`))
  (`|ExecutionSequence`
    (:`then_0`
      (`GameplayStatics.PlaySoundAtLocation` (`self.Open Door`) (`self.K2_GetActorLocation`) (struct) 1.0 1.0 0.0 null null null)
      (bind (_direction _lerpvalue) (`Timeline|MoveDoors`)
        (:`Update`
          (`SceneComponent.K2_SetRelativeLocation` _leftdoor (`KismetMathLibrary.VLerp` (`SceneComponent.RelativeLocation` _leftdoor) (132.0 0.0 0.0) _lerpvalue) false false)
          (`SceneComponent.K2_SetRelativeLocation` _rightdoor (`KismetMathLibrary.VLerp` (`SceneComponent.RelativeLocation` _rightdoor) (-132.0 0.0 0.0) _lerpvalue) false false))
        (:`Finished`
          (`|ExecutionSequence`
            (:`then_0`
              (`PrimitiveComponent.SetCollisionResponseToAllChannels` (`self.LeftDoor`) "ECR_Ignore"))
            (:`then_1`
              (`PrimitiveComponent.SetCollisionResponseToAllChannels` (`self.RightDoor`) "ECR_Ignore"))))))))

(fn `UserConstructionScript`)
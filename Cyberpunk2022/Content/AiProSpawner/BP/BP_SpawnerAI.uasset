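; Wave spawner that places random AI classes at random navmesh-reachable points around spawn points, with optional trigger-driven spawns.
; Game start launches waves that grow with the wave number, resuming from and saving the last wave in the game instance.
; A delayed polling loop counts living AI, respawns losses up to a per-wave limit, and starts the next wave once all die.
; Wave changes notify BP_NotificationService and switch music through the game state.
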(event `Trigger Spawn`
  (params (`Number to spawn` :type Integer) (Trigger :type "/Game/AiProSpawner/BP/BP_Trigger_Spawn Object Reference") (`Ai to spawn` :type "Array of Actor Class Reference") (`Delay before spawn ai` :type "Float (double-precision)"))
  ;[0 0 0] On Trigger Spawn AI
  (if (`self.SpawnAI On Trigger?`)
    (set `self.Trigger` Trigger)
    (`KismetSystemLibrary.Delay` `Delay before spawn ai`)
    (`self.Spawn AI Trigger` `Number to spawn` `Ai to spawn`)))

(event `self.ReceiveBeginPlay`
  ;[0 0 0] Event begin play and start
  ;;[0 0 0] Event begin play
  (bind _asbp_my_game_instance (cast `/Game/FirstPersonCPP/SaveSystem/BP_MyGameInstance` (`GameplayStatics.GetGameInstance`)))
  (bind _output_get (set `self.MyGameInstance` _asbp_my_game_instance))
  (set `self.Waves` (`/Game/FirstPersonCPP/SaveSystem/BP_SaveGame.LastWave` (`/Game/FirstPersonCPP/SaveSystem/BP_MyGameInstance.SaveGameData` _output_get)))
  (bind _output_get_2 (set `self.Limit of Ai respawn` (+ (`self.Number Of AI To Spawn`) (* (`self.Waves`) (`self.Number of ai add to next waves`)))))
  (`KismetSystemLibrary.PrintString` (`KismetStringLibrary.Conv_IntToString` _output_get_2) true true (struct :`R` 1.0 :`G` 0.820607 :`A` 1.0))
  (bind _returnvalue (`GameplayStatics.GetActorOfClass` "/Game/FirstPersonCPP/Services/BP_NotificationService.BP_NotificationService_C"))
  (set `self.NotificationService` _returnvalue)
  (`self.StartingServer`)
  (add `/Game/FirstPersonCPP/Services/BP_NotificationService.OnStartGame` (`self.NotificationService`) (delegate `OnStartGame_Event_0`)))

(event `OnStartGame_Event_0`
  (bind _delay_for_the_next_waves (`self.Delay for the next waves`))
  ;[0 0 0] Event begin play and start
  ;;[0 0 0] Event begin play
  (`/Game/FirstPersonCPP/Services/BP_NotificationService.OnEnemyIncoming` (`self.NotificationService`) _delay_for_the_next_waves)
  (`KismetSystemLibrary.Delay` _delay_for_the_next_waves)
  (`self.First Wave`))

(event `Respawn`
  ;[0 0 0] Waves system and respawn
  ;;[0 0 0] Respawn ai
  (if (<= (`self.Limit of Ai respawn`) 0)
    (`KismetSystemLibrary.Delay` 0.1)
    (`self.Check how many ai is alive`)
    (else
      (`KismetSystemLibrary.Delay` (`self.Delay For Respawn`))
      (`KismetSystemLibrary.PrintString` "respawn")
      (`self.Spawn AI` 1)
      (`/Engine/EditorBlueprintResources/StandardMacros.DecrementInt` (`self.Limit of Ai respawn`)))))

(event `StartWaves`
  ;[0 0 0] Event begin play and start
  ;;[0 0 0] Start spawner
  (if (== (`self.Waves`) 0) :!label _label
    (message `/Game/FirstPersonCPP/Blueprints/BPI_Music.ChangeMusicState` (`GameplayStatics.GetGameState`) 2.0)
    (else
      (`KismetSystemLibrary.Delay` (`self.Delay Before Spawn`))
      (`self.First Wave`))))

(event `StartingServer`
  ;[0 0 0] Event begin play and start
  ;;[0 0 0] Start spawner
  (`/Engine/EditorBlueprintResources/StandardMacros.DoOnce` false
    (:`Completed`
      (goto _label))))

(event `Check how many ai is alive`
  ;[0 0 0] Waves system and respawn
  ;;[0 0 0] Check ai alive and start wave or respawn ai
  (bind _all_dead_ (`self.Check Ai Alive`))
  (if (`self.WavesStarting?`)
    (if _all_dead_
      (if (`self.Stop Waves`)
        (`KismetSystemLibrary.Delay` 0.1)
        (`self.Check how many ai is alive`)
        (else
          (`/Game/FirstPersonCPP/Services/BP_NotificationService.OnWaveCompleted` (`self.NotificationService`) (`self.Waves`))
          (`self.Start a wave`)))
      (elif (`self.NewVar_0`)
        (if (< (`self.All AI Alive`) (+ (`self.Number Of AI To Spawn`) (* (- (`self.Waves`) 1) (`self.Number of ai add to next waves`))))
          (`self.Respawn`)
          (else
            (`KismetSystemLibrary.Delay` 1.0 :!label _label_2)
            (`self.Check how many ai is alive`)))
        (else
          (goto _label_2))))))

(event `First Wave`
  (bind _mygameinstance (`self.MyGameInstance`))
  (bind _waves (`self.Waves`))
  (bind _notificationservice (`self.NotificationService`))
  ;[0 0 0] Waves system and respawn
  ;;[0 0 0] Start a wave
  (set `self.WavesStarting?` true)
  (bind _number_ai_to_spawn (`self.How many spawn ai wave`))
  (bind _spawn_ai (`self.Spawn Wave` _number_ai_to_spawn))
  (if _spawn_ai
    (`/Game/FirstPersonCPP/Services/BP_NotificationService.OnEnemyIncoming` _notificationservice 0.0)
    (set `/Game/FirstPersonCPP/SaveSystem/BP_SaveGame.LastWave` _waves (`/Game/FirstPersonCPP/SaveSystem/BP_MyGameInstance.SaveGameData` _mygameinstance) :!label _label_3)
    (set `self.Waves` (+ _waves 1))
    (`/Game/FirstPersonCPP/SaveSystem/BP_MyGameInstance.SavePlayerData` _mygameinstance)
    (`/Game/FirstPersonCPP/SaveSystem/BP_MyGameInstance.SaveGame` _mygameinstance)
    (message `/Game/FirstPersonCPP/Blueprints/BPI_Music.ChangeMusicState` (`GameplayStatics.GetGameState`) 1.0)
    (if (>= (`self.Number ai to spawn Left`) 1) :!label _label_4
      (`KismetSystemLibrary.Delay` (`self.Delay between each ai spawn`))
      (bind _spawn_ai__ (`self.Spawn ai wave`))
      (if _spawn_ai__
        (goto _label_4)
        (else
          (set `self.NewVar_0` true)
          (`self.Check how many ai is alive`))))
    (else
      (`/Game/FirstPersonCPP/Services/BP_NotificationService.OnWaveCompleted` _notificationservice (`self.Number of waves`))
      (`/Game/FirstPersonCPP/Services/BP_NotificationService.OnAllWaveCompleted` _notificationservice)
      (message `/Game/FirstPersonCPP/Blueprints/BPI_Music.ChangeMusicState` (`GameplayStatics.GetGameState`) 3.0))))

(event `Start a wave`
  (bind _delay_for_the_next_waves (`self.Delay for the next waves`))
  ;[0 0 0] Waves system and respawn
  (bind _output_get (set `self.Limit of Ai respawn` (+ (`self.Number Of AI To Spawn`) (* (`self.Waves`) (`self.Number of ai add to next waves`)))))
  ;;[0 0 0] Start a wave
  (`KismetSystemLibrary.PrintString` (`KismetStringLibrary.Conv_IntToString` _output_get) true true (struct :`R` 1.0 :`B` 0.024691 :`A` 1.0))
  (set `self.NewVar_0` false)
  (if (not (`self.Stop Waves`))
    (bind _start_a_wave__ (`self.Check if start a wave`))
    (if _start_a_wave__
      (message `/Game/FirstPersonCPP/Blueprints/BPI_Music.ChangeMusicState` (`GameplayStatics.GetGameState`) 2.0)
      (`/Game/FirstPersonCPP/Services/BP_NotificationService.OnEnemyIncoming` (`self.NotificationService`) _delay_for_the_next_waves)
      (`KismetSystemLibrary.Delay` _delay_for_the_next_waves)
      (bind _number_ai_to_spawn (`self.How many spawn ai wave`))
      (bind _spawn_ai (`self.Spawn Wave` _number_ai_to_spawn))
      (if _spawn_ai
        (goto _label_3))
      (else
        (set `self.Stop Waves` true)
        (`KismetSystemLibrary.Delay` 0.5)
        (`self.Check how many ai is alive`)))))

(fn `Check Ai Alive`
  (returns (`All Dead?` :type Boolean))
  (set `self.All AI Alive` 0)
  (set `self.one is alive ?` false)
  (for _array_element (`self.All Ai Spawn`)
    ;[1 0.2135 0.2135] Cast you AI Parent
    (`/Engine/EditorBlueprintResources/StandardMacros.IsValid` _array_element
      (:`Is Valid`
        (bind _asbot_master (cast `/Game/FirstPersonCPP/AI/BotMaster/BotMaster` _array_element))
        (if (not (`/Game/FirstPersonCPP/AI/BotMaster/BotMaster.isDead` _asbot_master))
          (set `self.All AI Alive` (+ (`self.All AI Alive`) 1))
          (set `self.one is alive ?` true)))))
  (if (`self.one is alive ?`)
    (set `self.All dead?` false)
    (return false)
    (elif (<= (`self.Number ai to spawn Left`) 0)
      (set `self.All dead?` true)
      (return true)
      (else
        (set `self.All dead?` false)
        (return false)))))

(fn `Check if start a wave`
  (returns (`Start a wave ?` :type Boolean))
  (bind _mygameinstance (`self.MyGameInstance`))
  (if (`self.Inifnite Waves?`)
    (return true)
    (elif (>= (`self.Waves`) (`self.Number of waves`))
      (set `/Game/FirstPersonCPP/SaveSystem/BP_SaveGame.LastWave` (+ (`self.Waves`) 1) (`/Game/FirstPersonCPP/SaveSystem/BP_MyGameInstance.SaveGameData` _mygameinstance))
      (`/Game/FirstPersonCPP/SaveSystem/BP_MyGameInstance.SavePlayerData` _mygameinstance)
      (`/Game/FirstPersonCPP/SaveSystem/BP_MyGameInstance.SaveGame` _mygameinstance)
      (`/Game/FirstPersonCPP/Services/BP_NotificationService.OnAllWaveCompleted` (`self.NotificationService`))
      (message `/Game/FirstPersonCPP/Blueprints/BPI_Music.ChangeMusicState` (`GameplayStatics.GetGameState`) 3.0)
      (return false)
      (else
        (return true)))))

(fn `How many spawn ai wave`
  (returns (`Number ai to spawn` :type Integer))
  (if (> (+ (`self.Number Of AI To Spawn`) (`self.Number of ai add to next waves`)) (`self.Limit Of The Max AI`))
    (return (`self.Limit Of The Max AI`))
    (else
      (return (+ (`self.Number Of AI To Spawn`) (* (`self.Number of ai add to next waves`) (`self.Waves`)))))))

(fn `Spawn AI`
  (params (`Number of ai` :type Integer))
  (bind _class_of_actor_to_spawn (`self.Class Of Actor To Spawn`))
  (bind _spawn_points (`self.Spawn Points`))
  (bind _output (`|GetArrayItem` _spawn_points (`KismetMathLibrary.RandomIntegerInRange` 0 (`KismetArrayLibrary.Array_LastIndex` _spawn_points))))
  (bind (_returnvalue_x _returnvalue_y _returnvalue_z) (`KismetMathLibrary.BreakVector` (`self.K2_GetActorLocation` _output)))
  (bind _randomlocation (`NavigationSystemV1.K2_GetRandomReachablePointInRadius` (`KismetMathLibrary.MakeVector` _returnvalue_x _returnvalue_y _returnvalue_z) (`/Game/AiProSpawner/BP/BP_SpawnPoint.Radius Of Spawner` _output) null null))
  (set `self.Number ai to spawn Left` `Number of ai`)
  (for _ (range 1 (+ `Number of ai` 1))
    (bind _returnvalue (`|SpawnActorFromClass` (`|GetArrayItem` _class_of_actor_to_spawn (`KismetMathLibrary.RandomIntegerInRange` 0 (`KismetArrayLibrary.Array_LastIndex` _class_of_actor_to_spawn))) (`KismetMathLibrary.MakeTransform` (`KismetMathLibrary.MakeVector` (.x _randomlocation) (.y _randomlocation) (+ (.z _randomlocation) 50.0))) "AdjustIfPossibleButAlwaysSpawn" "OverrideRootScale" null null))
    (`KismetArrayLibrary.Array_Add` (`self.All Ai Spawn`) _returnvalue)
    (set `self.Number ai to spawn Left` (- (`self.Number ai to spawn Left`) 1)))
  (`self.Check how many ai is alive`))

(fn `Spawn AI Trigger`
  (params (`Number of ai` :type Integer) (`Ai To Spawn` :type "Array of Actor Class Reference"))
  (bind _spawnpoints (`/Game/AiProSpawner/BP/BP_Trigger_Spawn.SpawnPoints` (`self.Trigger`)))
  (bind _output (`|GetArrayItem` _spawnpoints (`KismetMathLibrary.RandomIntegerInRange` 0 (`KismetArrayLibrary.Array_LastIndex` _spawnpoints))))
  (bind (_returnvalue_x _returnvalue_y _returnvalue_z) (`KismetMathLibrary.BreakVector` (`self.K2_GetActorLocation` _output)))
  (bind _randomlocation (`NavigationSystemV1.K2_GetRandomReachablePointInRadius` (`KismetMathLibrary.MakeVector` _returnvalue_x _returnvalue_y _returnvalue_z) (`/Game/AiProSpawner/BP/BP_SpawnPoint.Radius Of Spawner` _output) null null))
  (for _ (range 1 (+ `Number of ai` 1))
    (`|SpawnActorFromClass` (`|GetArrayItem` `Ai To Spawn` (`KismetMathLibrary.RandomIntegerInRange` 0 (`KismetArrayLibrary.Array_LastIndex` `Ai To Spawn`))) (`KismetMathLibrary.MakeTransform` (`KismetMathLibrary.MakeVector` (.x _randomlocation) (.y _randomlocation) (+ (.z _randomlocation) 50.0))) "AdjustIfPossibleButAlwaysSpawn" "OverrideRootScale" null null))
  (`self.Check how many ai is alive`))

(fn `Spawn ai wave`
  (returns (`spawn ai ?` :type Boolean))
  (bind _class_of_actor_to_spawn (`self.Class Of Actor To Spawn`))
  (bind _spawn_points (`self.Spawn Points`))
  (bind _output (`|GetArrayItem` _spawn_points (`KismetMathLibrary.RandomIntegerInRange` 0 (`KismetArrayLibrary.Array_LastIndex` _spawn_points))))
  (bind (_returnvalue_x _returnvalue_y _returnvalue_z) (`KismetMathLibrary.BreakVector` (`self.K2_GetActorLocation` _output)))
  (bind _randomlocation (`NavigationSystemV1.K2_GetRandomReachablePointInRadius` (`KismetMathLibrary.MakeVector` _returnvalue_x _returnvalue_y _returnvalue_z) (`/Game/AiProSpawner/BP/BP_SpawnPoint.Radius Of Spawner` _output) null null))
  (bind _returnvalue (`|SpawnActorFromClass` (`|GetArrayItem` _class_of_actor_to_spawn (`KismetMathLibrary.RandomIntegerInRange` 0 (`KismetArrayLibrary.Array_LastIndex` _class_of_actor_to_spawn))) (`KismetMathLibrary.MakeTransform` (`KismetMathLibrary.MakeVector` (.x _randomlocation) (.y _randomlocation) (+ (.z _randomlocation) 50.0))) "AdjustIfPossibleButAlwaysSpawn" "OverrideRootScale" null null))
  (`KismetArrayLibrary.Array_Add` (`self.All Ai Spawn`) _returnvalue)
  (bind _output_get (set `self.Number ai to spawn Left` (- (`self.Number ai to spawn Left`) 1)))
  (`self.Check how many ai is alive`)
  (return (>= _output_get 1)))

(fn `Spawn Wave`
  (params (`Number of ai` :type Integer))
  (returns (`Spawn ai` :type Boolean))
  (set `self.Number ai to spawn Left` `Number of ai`)
  (if (`self.Inifnite Waves?`)
    (return true)
    (elif (>= (`self.Waves`) (`self.Number of waves`))
      (set `self.Stop Waves` true)
      (return false)
      (else
        (return true)))))

(fn `UserConstructionScript`)
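; BP_SimpleAI_Parent is a simple AI pawn that chases players and ragdolls on death, apparently meant as a base class.
; Each tick while alive, it scans all BP_Player actors for the closest within a fixed range and re-issues AIMoveTo toward the stored target.
; Die runs once, also reachable through the Dead event: it enables mesh physics, disables capsule collision and destroys the actor after a delay.
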(event `self.ReceiveTick`
  (params (DeltaSeconds :type "Float (single-precision)"))
  ;[0 0 0] Ai follow player
  ;;[0 0 0] Event tick
  (if (not (`self.Dead?`))
    (set `self.Closet_PlayerDistance` 2000.0)
    ;;[0.3385 0.1005 0.1005] Put your player here
    (bind _outactors (`GameplayStatics.GetAllActorsOfClass` "/Game/AiProSpawner/BP/BP_Player.BP_Player_C"))
    ;;[0 0 0] Search The Closet Player
    (for _array_element _outactors
      (bind _returnvalue (`self.GetDistanceTo` _array_element self))
      (if (< _returnvalue (`self.Closet_PlayerDistance`))
        (set `self.Closet_PlayerDistance` _returnvalue)
        (set `self.Closet_PlayerCharacer` _array_element)))
    (`self.Ai move`)))

(event `Ai move`
  ;[0 0 0] Ai follow player
  ;;[0 0 0] Ai move
  (`|AIMoveTo` self (0.0 0.0 0.0) (`self.Closet_PlayerCharacer`)))

(event `Dead`
  ;[0 0 0] Die
  (`self.Die`))

(event `Die`
  ;[0 0 0] Die
  (`/Engine/EditorBlueprintResources/StandardMacros.DoOnce` false
    (:`Completed`
      (`PrimitiveComponent.SetSimulatePhysics` (`self.Mesh`) true)
      (set `self.Dead?` true)
      (`PrimitiveComponent.SetCollisionEnabled` (`self.CapsuleComponent`) "NoCollision")
      (`KismetSystemLibrary.Delay` 4.9)
      (`self.K2_DestroyActor`))))

(fn `UserConstructionScript`)
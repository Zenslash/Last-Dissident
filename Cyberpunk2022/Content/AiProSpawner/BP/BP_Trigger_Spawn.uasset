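; Trigger volume that, on its first overlap by BP_Player, tells the level's BP_SpawnerAI to spawn AI or start waves.
; It uses the first spawner found, calling StartWaves if its own StartWaves flag is set, otherwise TriggerSpawn with its count, AI and delay settings if the spawner allows SpawnAIOnTrigger.
; The construction script applies the trigger's configurable scale, location and in-game visibility.
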(event `self.Trigger.OnComponentBeginOverlap`
  (params (OverlappedComponent :type "PrimitiveComponent Object Reference") (OtherActor :type "Actor Object Reference") (OtherComp :type "PrimitiveComponent Object Reference") (OtherBodyIndex :type Integer) (bFromSweep :type Boolean) (SweepResult :type "HitResult Structure (by ref)"))
  ;[0 0 0] On trigger spawn ai
  ;;[1 0.125 0.125] Cast your player
  (cast `/Game/AiProSpawner/BP/BP_Player` OtherActor)
  (`/Engine/EditorBlueprintResources/StandardMacros.DoOnce` false
    (:`Completed`
      (bind _outactors (`GameplayStatics.GetAllActorsOfClass` "/Game/AiProSpawner/BP/BP_SpawnerAI.BP_SpawnerAI_C"))
      (bind _output (`|GetArrayItem` _outactors))
      (if (`/Game/AiProSpawner/BP/BP_SpawnerAI.SpawnAI On Trigger?` _output)
        (if (not (`self.StartWaves?`))
          (`/Game/AiProSpawner/BP/BP_SpawnerAI.Trigger Spawn` _output (`self.Number Ai To Spawn`) self (`self.Ai To Spawn`) (`self.Delay before spawn`))
          (else
            (`/Game/AiProSpawner/BP/BP_SpawnerAI.StartWaves` _output :!label _label)))
        (elif (not (not (`self.StartWaves?`)))
          (goto _label))))))

(fn `UserConstructionScript`
  ;[0 0 0] set trigger scale
  (`SceneComponent.SetWorldScale3D` (`self.Trigger`) (`self.Trigger Scale`))
  ;[0 0 0] Set the location of the trigger
  (`SceneComponent.K2_SetRelativeLocation` (`self.Trigger`) (`self.Location Of The Trigger`) false false)
  ;[0 0 0] See the trigger in game ?
  (if (`self.See the trigger in game?`)
    (`SceneComponent.SetHiddenInGame` (`self.Trigger`) false false)
    (else
      (`SceneComponent.SetHiddenInGame` (`self.Trigger`) true false))))